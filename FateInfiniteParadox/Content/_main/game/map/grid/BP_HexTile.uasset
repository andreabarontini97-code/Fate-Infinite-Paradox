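; BP_HexTile is a single tile on the hex grid map, holding its terrain type data and labels for its coordinates and degrees.
; The Construction Script uses the TileType enum name as a data table row key, caches that row in TileTypeData and prints an error when none matches.
; On a match it also fills text labels with Q/R coordinates and current/target degrees.
; GetTileModifier exposes the cached stat modifier.
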(fn `GetTileModifier`
  (returns (StatModifier :type "/Game/_main/core/stats/data/F_Stats Structure"))
  (bind (_tiletypedata_tiletype _tiletypedata_displayname _tiletypedata_movecost _tiletypedata_statmodifier) (break `/Game/_main/game/map/data/F_TileTypeData` (`self.TileTypeData`)))
  (return _tiletypedata_statmodifier))

(fn `UserConstructionScript`
  (bind (_q _r) (break `/Game/_main/game/map/data/F_HexCoord` (`self.HexCoord`)))
  (bind (_coord _neighbours _currentdegree _targetdegree) (break `/Game/_main/game/map/data/F_HexTileData` (`self.HexTileData`)))
  (bind _returnvalue (`|GetDataTableRow` (`self.TileTypeDataTable`) (`KismetStringLibrary.Conv_StringToName` (`|GetEnumeratorNameAsString` (`self.TileType`))))
    (:`then`
      (bind (_tiletype _displayname _movecost _statmodifier _sprite _description) (break `/Game/_main/game/map/data/F_TileTypeData` _returnvalue))
      (set `self.TileTypeData` (make `/Game/_main/game/map/data/F_TileTypeData` _tiletype _displayname _movecost _statmodifier _sprite _description))
      (`TextRenderComponent.K2_SetText` (`self.HexCoords`) (`|FormatText` "(Q={Q}, R={R})" _q _r))
      (`TextRenderComponent.K2_SetText` (`self.Degrees`) (`|FormatText` "Cur {c} Tar {t}" _currentdegree _targetdegree)))
    (:`RowNotFound`
      (`KismetSystemLibrary.PrintString` "Row was not found in the tile type data table" true true (struct :`R` 1.0 :`G` 0.039027 :`A` 1.0) 10.0))))