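; Actor that procedurally builds a random hex-tile map on BeginPlay and spawns a BP_HexTile per axial coordinate.
; Growth starts at the origin and expands random frontier tiles, respecting each tile's target neighbour count drawn from a weighted DataTable.
; Generation stops at the target size, on an empty frontier, or after too many failed placements.
; Optional refinement pairs under-connected frontier tiles, moving one beside the other.
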(event `self.ReceiveBeginPlay`
  (`self.GenerateMap` 16)
  (`self.SpawnTiles`))

(fn `AddNewTile`
  (params (Coord :type "/Game/_main/game/map/data/F_HexCoord Structure"))
  (returns (Successfull :type Boolean))
  (bind _f_hextiledata (make `/Game/_main/game/map/data/F_HexTileData` :`Coord` Coord :`CurrentDegree` (`KismetArrayLibrary.Array_Length` (`/Game/_main/game/map/utils/BPFL_HexMath.GetOccupiedNeighbours` Coord (`self.TilesMap`))) :`TargetDegree` (`self.SampleTargetDegree`)))
  (bind (_coord _neighbours _currentdegree _targetdegree) (break `/Game/_main/game/map/data/F_HexTileData` _f_hextiledata))
  (if (> _currentdegree _targetdegree)
    (return false)
    (else
      (`BlueprintMapLibrary.Map_Add` (`self.TilesMap`) Coord _f_hextiledata)
      (`KismetArrayLibrary.Array_Add` (`self.Frontier`) Coord)
      (return true))))

(fn `AreThereFreeNeighbours`
  (params (ExpandTileFreeNeighbours :type "Array of /Game/_main/game/map/data/F_HexCoord Structure"))
  (returns (`There are` :type Boolean))
  (return (> (`KismetArrayLibrary.Array_Length` ExpandTileFreeNeighbours) 0)))

(fn `CompleteGeneration`
  (params (FailureCounter :type Integer))
  (if (>= FailureCounter (`self.MaxFailures`))
    (`KismetSystemLibrary.PrintText` (`|FormatText` "Generation completed as failure are {F}, with max allowed {M}" FailureCounter (`self.MaxFailures`)) true true (struct :`R` 1.0 :`G` 0.039027 :`A` 1.0) 200.0)
    (else
      (`KismetSystemLibrary.PrintText` (`|FormatText` "Completed as reached the target num of tiles, with failures {fail}" FailureCounter) true true (struct :`G` 0.66 :`B` 1.0 :`A` 1.0) 200.0))))

(fn `GenerateMap`
  (params (TargetTileNum :type Integer))
  (locals (CurrentTileCount :type Integer) (ExpandCoord :type "/Game/_main/game/map/data/F_HexCoord Structure") (ExpandTileData :type "/Game/_main/game/map/data/F_HexTileData Structure") (ExpandTileFreeNeighbours :type "Array of /Game/_main/game/map/data/F_HexCoord Structure") (FailureCounter :type Integer))
  ; Initialization
  (set `local.FailureCounter` 0)
  (set `local.CurrentTileCount` 0)
  (`self.InitializeMap`)
  ; Create Origin in (0,0)
  (bind _successfull (`self.AddNewTile` (make `/Game/_main/game/map/data/F_HexCoord` 0)))
  (if _successfull
    (`/Engine/EditorBlueprintResources/StandardMacros.IncrementInt` (`local.CurrentTileCount`)
      (:`  `
        (while (`self.ShouldGenerationContinue` (`local.CurrentTileCount`) (`local.TargetTileNum`) (`local.FailureCounter`))
          (bind _it_is (`self.IsFrontierEmpty`))
          (if _it_is
            ; Frontier is empty
            (`KismetSystemLibrary.RaiseScriptError` "Frontier is empty before reaching the num tiles goal")
            (return)
            (else
              (bind (_coord _tiledata) (`self.GetRandomFrontierTileCoord`))
              (set `local.ExpandCoord` _coord)
              (bind _output_get (set `local.ExpandTileData` _tiledata))
              (bind _it_is_2 (`self.IsTileAlreadyFull` _output_get))
              (if _it_is_2
                ; ExpandTileReachedTargetNeighbours
                (`KismetArrayLibrary.Array_RemoveItem` (`self.Frontier`) (`local.ExpandCoord`))
                (else
                  (bind _output_get_2 (set `local.ExpandTileFreeNeighbours` (`/Game/_main/game/map/utils/BPFL_HexMath.GetFreeNeighboursCoords` (`local.ExpandCoord`) (`self.TilesMap`))))
                  (bind _there_are (`self.AreThereFreeNeighbours` _output_get_2))
                  (if _there_are
                    (bind (_freeneighbour _foundneighbour) (`self.GetRandomFreeNeighbour` (`local.ExpandTileFreeNeighbours`) (`self.TilesMap`)))
                    (if _foundneighbour
                      (bind _successfull_2 (`self.AddNewTile` _freeneighbour))
                      (if _successfull_2
                        (`/Engine/EditorBlueprintResources/StandardMacros.IncrementInt` (`local.CurrentTileCount`)
                          (:`  `
                            (`self.UpdateAllCurrentDegrees` _freeneighbour)
                            (`self.LogStatusOfGeneration` (`local.CurrentTileCount`))))
                        (else
                          ; Inserting a new tile would break the new tile target neighbours
                          (`/Engine/EditorBlueprintResources/StandardMacros.IncrementInt` (`local.FailureCounter`))))
                      (else
                        ; Inserting a new tile would break the current target neighbours for at least one tile
                        (`/Engine/EditorBlueprintResources/StandardMacros.IncrementInt` (`local.FailureCounter`))))
                    (else
                      ; ExpandTile has no free neighbours
                      (`KismetArrayLibrary.Array_RemoveItem` (`self.Frontier`) (`local.ExpandCoord`)))))))))
        (if (`self.DoRefinement`)
          (`self.RefineMap`))
        ; Generation Completed
        (`self.CompleteGeneration` (`local.FailureCounter`))))
    (else
      (`KismetSystemLibrary.PrintString` "Error in generating the first tile" true true (struct :`R` 1.0 :`G` 0.039027 :`A` 1.0)))))

(fn `GetRandomFreeNeighbour`
  (params (FreeNeighbours :type "Array of /Game/_main/game/map/data/F_HexCoord Structure") (TileMap :type "Map of /Game/_main/game/map/data/F_HexCoord Structure to /Game/_main/game/map/data/F_HexTileData Structure"))
  (returns (FreeNeighbour :type "/Game/_main/game/map/data/F_HexCoord Structure") (FoundNeighbour :type Boolean))
  (locals (found :type Boolean) (freeNeighbourCoord :type "/Game/_main/game/map/data/F_HexCoord Structure") (OccupiedNeighbours :type "Array of /Game/_main/game/map/data/F_HexCoord Structure"))
  (bind _output_get (set `local.freeNeighbourCoord` (`|GetArrayItem` FreeNeighbours (`KismetMathLibrary.RandomIntegerInRange` 0 (- (`KismetArrayLibrary.Array_Length` FreeNeighbours) 1)))))
  (set `local.found` true)
  (bind _output_get_2 (set `local.OccupiedNeighbours` (`/Game/_main/game/map/utils/BPFL_HexMath.GetOccupiedNeighbours` _output_get TileMap)))
  (for _array_element _output_get_2
    (bind _it_is (`self.IsTileAlreadyFull` (`BlueprintMapLibrary.Map_Find` (`local.TileMap`) _array_element)))
    (if _it_is
      (set `local.found` false)
      (break)))
  (return (`local.freeNeighbourCoord`) (`local.found`)))

(fn `GetRandomFrontierTileCoord`
  (returns (Coord :type "/Game/_main/game/map/data/F_HexCoord Structure") (TileData :type "/Game/_main/game/map/data/F_HexTileData Structure"))
  (bind _output (`|GetArrayItem` (`self.Frontier`) (`KismetMathLibrary.RandomIntegerInRange` 0 (- (`KismetArrayLibrary.Array_Length` (`self.Frontier`)) 1))))
  (bind (_value _returnvalue) (`BlueprintMapLibrary.Map_Find` (`self.TilesMap`) _output))
  (if _returnvalue
    (return _output _value)
    (else
      (`KismetSystemLibrary.RaiseScriptError` "Frontier tile not found in tiles map")
      (`KismetSystemLibrary.QuitGame` null "Quit"))))

(fn `HexToWorld`
  (params (HexCoord :type "/Game/_main/game/map/data/F_HexCoord Structure"))
  (returns (WorldCoord :type "Vector Structure"))
  (bind (_q _r) (break `/Game/_main/game/map/data/F_HexCoord` HexCoord))
  (return (`KismetMathLibrary.MakeVector` (* (* (`self.HexSize`) 1.5) _q) (* (+ _r (/ (`KismetMathLibrary.Conv_IntToDouble` _q) 2.0)) (* (`self.HexSize`) (`KismetMathLibrary.Sqrt` 3.0))))))

(fn `InitializeMap`
  (`BlueprintMapLibrary.Map_Clear` (`self.TilesMap`))
  (`KismetArrayLibrary.Array_Clear` (`self.Frontier`)))

(fn `IsFrontierEmpty`
  (returns (`It is` :type Boolean))
  (return (== (`KismetArrayLibrary.Array_Length` (`self.Frontier`)) 0)))

(fn `IsTileAlreadyFull`
  (params (F_HexTileData :type "/Game/_main/game/map/data/F_HexTileData Structure (by ref)"))
  (returns (`It is` :type Boolean))
  (bind (_coord _neighbours _currentdegree _targetdegree) (break `/Game/_main/game/map/data/F_HexTileData` F_HexTileData))
  (return (>= _currentdegree _targetdegree)))

(fn `LogStatusOfGeneration`
  (params (c :type Integer))
  (`KismetSystemLibrary.PrintText` (`|FormatText` "TileMap len {t}, frontier len {f}, tile count {c}" (`BlueprintMapLibrary.Map_Length` (`self.TilesMap`)) (`KismetArrayLibrary.Array_Length` (`self.Frontier`)) c) true true (struct :`G` 0.66 :`B` 1.0 :`A` 1.0) 200.0))

(fn `RefineMap`
  (locals (ToBeFixedList :type "Array of /Game/_main/game/map/data/F_HexCoord Structure") (CoordWhereToMove :type "/Game/_main/game/map/data/F_HexCoord Structure"))
  (bind (_coordwheretomove_q _coordwheretomove_r) (break `/Game/_main/game/map/data/F_HexCoord` (`local.CoordWhereToMove`)))
  (`KismetArrayLibrary.Array_Clear` (`local.ToBeFixedList`))
  (for _array_element (`self.Frontier`)
    (bind (_coord _neighbours _currentdegree _targetdegree) (break `/Game/_main/game/map/data/F_HexTileData` (`BlueprintMapLibrary.Map_Find` (`self.TilesMap`) _array_element)))
    (if (and (<= _currentdegree 2) (< _currentdegree _targetdegree))
      (`KismetArrayLibrary.Array_Add` (`local.ToBeFixedList`) _array_element)))
  (if (> (`KismetArrayLibrary.Array_Length` (`local.ToBeFixedList`)) 1)
    (`KismetSystemLibrary.PrintString` "Starting refinement of map" true true (struct :`G` 0.66 :`B` 1.0 :`A` 1.0) 200.0)
    (for (_array_element_2 _array_index) (`local.ToBeFixedList`)
      (if (== (mod _array_index 2) 0)
        (bind _freeneighbourscoords (`/Game/_main/game/map/utils/BPFL_HexMath.GetFreeNeighboursCoords` _array_element_2 (`self.TilesMap`)))
        (set `local.CoordWhereToMove` (`|GetArrayItem` _freeneighbourscoords (`KismetMathLibrary.RandomIntegerInRange` 0 (- (`KismetArrayLibrary.Array_Length` _freeneighbourscoords) 1))))
        (else
          (bind (_coord_2 _neighbours_2 _currentdegree_2 _targetdegree_2) (break `/Game/_main/game/map/data/F_HexTileData` (`BlueprintMapLibrary.Map_Find` (`self.TilesMap`) _array_element_2)))
          (`BlueprintMapLibrary.Map_Add` (`self.TilesMap`) (`local.CoordWhereToMove`) (make `/Game/_main/game/map/data/F_HexTileData` (`local.CoordWhereToMove`) _neighbours_2 _currentdegree_2 _targetdegree_2))
          (`BlueprintMapLibrary.Map_Remove` (`self.TilesMap`) _array_element_2)
          (`self.UpdateAllCurrentDegrees` (`local.CoordWhereToMove`))
          (bind (_q _r) (break `/Game/_main/game/map/data/F_HexCoord` _array_element_2))
          (`KismetSystemLibrary.PrintText` (`|FormatText` "Moved tile that was in coord ({Qpre}, {Rpre}) in new coord ({Q}, {R})" _q _r _coordwheretomove_q _coordwheretomove_r) true true (struct :`G` 0.66 :`B` 1.0 :`A` 1.0) 200.0))))
    (`KismetSystemLibrary.PrintString` "Completed refinement" true true (struct :`G` 0.66 :`B` 1.0 :`A` 1.0) 200.0)
    (else
      (return))))

(fn `SampleTargetDegree`
  (returns (TargetDegree :type Integer))
  (locals (DegreeSampled :type Integer) (RandomNumber :type "Float (double-precision)"))
  (bind _tileneighboursdistribution (`self.TileNeighboursDistribution`))
  (set `local.DegreeSampled` 6)
  (set `local.RandomNumber` (`KismetMathLibrary.RandomFloat`))
  (bind _outrownames (`DataTableFunctionLibrary.GetDataTableRowNames` _tileneighboursdistribution))
  (for _array_element _outrownames
    (bind _returnvalue (`|GetDataTableRow` _tileneighboursdistribution _array_element)
      (:`then`
        (bind (_numofneighbours _weight) (break `/Game/_main/game/map/data/F_TileNeighboursWeight` _returnvalue))
        (if (< (`local.RandomNumber`) _weight)
          (set `local.DegreeSampled` _numofneighbours)
          (break)))
      (:`RowNotFound`
        (`KismetSystemLibrary.RaiseScriptError` "Row not Found in data table for sampling degree"))))
  (return (`local.DegreeSampled`)))

(fn `ShouldGenerationContinue`
  (params (CurrentTileCount :type Integer) (TargetTileNum :type Integer) (FailureCounter :type Integer))
  (returns (`It is` :type Boolean))
  (return (and (< CurrentTileCount TargetTileNum) (< FailureCounter (`self.MaxFailures`)))))

(fn `SpawnTiles`
  (bind _keys (`BlueprintMapLibrary.Map_Keys` (`self.TilesMap`)))
  (for _array_element _keys
    (bind _worldcoord (`self.HexToWorld` _array_element))
    (`|SpawnActorFromClass` "/Game/_main/game/map/grid/BP_HexTile.BP_HexTile_C" (`KismetMathLibrary.MakeTransform` _worldcoord) "Undefined" "MultiplyWithRoot" null _array_element (`BlueprintMapLibrary.Map_Find` (`self.TilesMap`) _array_element) null)))

(fn `UpdateAllCurrentDegrees`
  (params (NewTileCoord :type "/Game/_main/game/map/data/F_HexCoord Structure"))
  (locals (HexData :type "/Game/_main/game/map/data/F_HexTileData Structure") (Neighbours :type "Array of /Game/_main/game/map/data/F_HexCoord Structure"))
  (bind _occupiedneighbourscoords (`/Game/_main/game/map/utils/BPFL_HexMath.GetOccupiedNeighbours` NewTileCoord (`self.TilesMap`)))
  (bind (_coord _neighbours _currentdegree _targetdegree) (break `/Game/_main/game/map/data/F_HexTileData` (`BlueprintMapLibrary.Map_Find` (`self.TilesMap`) NewTileCoord)))
  (`BlueprintMapLibrary.Map_Add` (`self.TilesMap`) NewTileCoord (make `/Game/_main/game/map/data/F_HexTileData` _coord _occupiedneighbourscoords (`KismetArrayLibrary.Array_Length` _occupiedneighbourscoords) _targetdegree))
  (bind _output_get (set `local.Neighbours` (`/Game/_main/game/map/utils/BPFL_HexMath.GetNeighbours` NewTileCoord)))
  (for _array_element _output_get
    (bind (_value _returnvalue) (`BlueprintMapLibrary.Map_Find` (`self.TilesMap`) _array_element))
    (if _returnvalue
      (bind _output_get_2 (set `local.HexData` _value))
      (bind (_coord_2 _neighbours_2 _currentdegree_2 _targetdegree_2) (break `/Game/_main/game/map/data/F_HexTileData` _output_get_2))
      (bind _occupiedneighbourscoords_2 (`/Game/_main/game/map/utils/BPFL_HexMath.GetOccupiedNeighbours` _array_element (`self.TilesMap`)))
      (`BlueprintMapLibrary.Map_Add` (`self.TilesMap`) _array_element (make `/Game/_main/game/map/data/F_HexTileData` _coord_2 _occupiedneighbourscoords_2 (`KismetArrayLibrary.Array_Length` _occupiedneighbourscoords_2) _targetdegree_2))))
  (return))

(fn `UserConstructionScript`)