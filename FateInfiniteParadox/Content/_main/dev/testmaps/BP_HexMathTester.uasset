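; BP_HexMathTester is a dev test actor that exercises hex grid math functions on BeginPlay.
; A sequence runs checks on neighbour count, neighbour values, hex distance, free neighbours in a test tile map, and the direction list, using test coordinate variables.
; Results go to on-screen prints of axial Q/R coordinates and values; only the six-neighbour count is compared against an expected result, the rest are checked by eye.
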(event `self.ReceiveBeginPlay`
  (bind _neighbours (`/Game/_main/game/map/utils/BPFL_HexMath.GetNeighbours` (`self.TestCoordNeighbours`)))
  (`|ExecutionSequence`
    (:`then_0`
      ; Test1-NumberOfNeighbours
      (if (== (`KismetArrayLibrary.Array_Length` _neighbours) 6)
        (`KismetSystemLibrary.PrintString` "Number of neighbours is correctly 6" true true (struct :`R` 0.002573 :`G` 0.03125 :`B` 0.000163 :`A` 1.0))
        (else
          (`KismetSystemLibrary.PrintString` "Error, number of neighbours is not 6" true true (struct :`R` 1.0 :`G` 0.039027 :`A` 1.0)))))
    (:`then_1`
      ; Test2-ValuesOfNeighbours
      (for _array_element _neighbours
        (bind (_q _r) (break `/Game/_main/game/map/data/F_HexCoord` _array_element))
        (`KismetSystemLibrary.PrintString` (`KismetTextLibrary.Conv_TextToString` (`|FormatText` "(Q={Q}, R={R})" (`KismetStringLibrary.Conv_IntToString` _q) (`KismetStringLibrary.Conv_IntToString` _r))) true true (struct :`G` 0.66 :`B` 1.0 :`A` 1.0) 10.0))
      (`KismetSystemLibrary.PrintString` "Test completed!"))
    (:`then_2`
      ; Test3-HexDistance
      (`KismetSystemLibrary.PrintString` (`KismetTextLibrary.Conv_TextToString` (`|FormatText` "The distance is {distance}" (`/Game/_main/game/map/utils/BPFL_HexMath.HexDistance` (`self.TestCoordDistance_A`) (`self.TestCoordDistance_B`)))) true true (struct :`G` 0.66 :`B` 1.0 :`A` 1.0) 10.0))
    (:`then_3`
      ; TestGetFreeNeighbours
      (set `self.CachedFreeNeighbours` (`/Game/_main/game/map/utils/BPFL_HexMath.GetFreeNeighboursCoords` (`self.TestCoordFreeNeighbours`) (`self.TestTilesMapFreeNeighbours`)))
      (for _array_element_2 (`self.CachedFreeNeighbours`)
        (bind (_q_2 _r_2) (break `/Game/_main/game/map/data/F_HexCoord` _array_element_2))
        (`KismetSystemLibrary.PrintString` (`KismetTextLibrary.Conv_TextToString` (`|FormatText` "({Q}, {R})" _q_2 _r_2)) true true (struct :`G` 0.66 :`B` 1.0 :`A` 1.0) 10.0)))
    (:`then_4`
      ; Test Directions
      (for _array_element_3 (`/Game/_main/game/map/utils/BPFL_HexMath.GetHexDirections`)
        (bind (_q_3 _r_3) (break `/Game/_main/game/map/data/F_HexCoord` _array_element_3))
        (`KismetSystemLibrary.PrintString` (`KismetTextLibrary.Conv_TextToString` (`|FormatText` "Direction = ({Q}, {R})" _q_3 _r_3)) true true (struct :`G` 0.66 :`B` 1.0 :`A` 1.0) 30.0)))))

(fn `UserConstructionScript`)